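; Health component that tracks its owner's health, signals death and handles first aid kit pickups.
; It binds to the owner's point and radial damage events, subtracts damage and sends the clamped value to the owner through SendHealthToClientMessage.
; At zero or below it calls PlayerDeathMessage on the owner; the stored health itself is not clamped.
; An aid kit restores full health and is destroyed, only when health is below default.
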(event Custom|UseAidKit
  (params (AidKit :type BP%20Pickup%20Object%20Reference))
  ;[0 0 0] First Aid Kit
  (if (< (Variables|Default|GetHealth) (Variables|Default|GetDefaultHealth))
    (Variables|Default|SetHealth (Variables|Default|GetDefaultHealth))
    (Class|BPIMPCharacter|SendHealthtoClient(Message) (Variables|Default|GetPlayer) (Variables|Default|GetDefaultHealth))
    (Actor|DestroyActor AidKit)))

(event Custom|PointDamage
  (params (DamagedActor :type Actor%20Object%20Reference) (Damage :type Float%20%28single-precision%29) (InstigatedBy :type Controller%20Object%20Reference) (HitLocation :type Vector) (FHitComponent :type Primitive%20Component%20Object%20Reference) (BoneName :type Name) (ShotFromDirection :type Vector) (DamageType :type Damage%20Type%20Object%20Reference) (DamageCauser :type Actor%20Object%20Reference))
  (Variables|Default|SetHealth (- (Variables|Default|GetHealth) Damage))
  (Class|BPIMPCharacter|SendHealthtoClient(Message) (Variables|Default|GetPlayer) (Math|Float|Clamp(Float) (Variables|Default|GetHealth) 0.0 (Variables|Default|GetDefaultHealth)))
  (if (<= (Variables|Default|GetHealth) 0.0)
    (Class|BPIMPCharacter|PlayerDeath(Message) (Components|GetOwner))))

(event Custom|RadialDamage
  (params (DamagedActor :type Actor%20Object%20Reference) (Damage :type Float%20%28single-precision%29) (DamageType :type Damage%20Type%20Object%20Reference) (Origin :type Vector) (HitInfo :type Hit%20Result%20Structure) (InstigatedBy :type Controller%20Object%20Reference) (DamageCauser :type Actor%20Object%20Reference))
  (Variables|Default|SetHealth (- (Variables|Default|GetHealth) Damage))
  (Class|BPIMPCharacter|SendHealthtoClient(Message) (Variables|Default|GetPlayer) (Math|Float|Clamp(Float) (Variables|Default|GetHealth) 0.0 (Variables|Default|GetDefaultHealth)))
  (if (<= (Variables|Default|GetHealth) 0.0)
    (Class|BPIMPCharacter|PlayerDeath(Message) (Components|GetOwner))))

(event EventBeginPlay
  (bind _returnvalue (Components|GetOwner))
  (EventDispatchers|BindEventtoOnTakePointDamage _returnvalue (delegate Custom|PointDamage))
  (EventDispatchers|BindEventtoOnTakeRadialDamage _returnvalue (delegate Custom|RadialDamage))
  (Variables|Default|SetHealth (Variables|Default|GetDefaultHealth))
  (Variables|Default|SetPlayer (Components|GetOwner)))