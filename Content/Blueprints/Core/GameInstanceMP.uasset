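; Multiplayer game instance that hosts Advanced Sessions games, handles accepted session invites and stores the player's Steam info.
; HOST_SESSION creates a session tagged with name, map and game mode, using the same count for public and private connections, then opens the map as a listen server.
; Accepted invites join the session directly, while received invites do nothing and session creation results are only printed as debug strings.
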(event Custom|HOST_SESSION
  (params (PublicConnections :type Integer) (bUseLAN :type Boolean) (SessionName :type String) (MapName :type String) (GameMode :type String))
  ;[0 0 0] HOST SESSION
  (|AdvancedSession (Utilities|Array|MakeArray (Class|AdvancedSessionsLibrary|MakeLiteralSessionPropertyString "SessionName" SessionName) (Class|AdvancedSessionsLibrary|MakeLiteralSessionPropertyString "MapName" MapName) (Class|AdvancedSessionsLibrary|MakeLiteralSessionPropertyString "GameMode" GameMode)) (Game|GetPlayerController 0) PublicConnections PublicConnections bUseLAN true false true true false false false true
    (:OnSuccess
      (Development|PrintString "Success session creation" true true "(R=0.000000,G=1.000000,B=0.000000,A=1.000000)" 1e+01)
      (Game|OpenLevel(byName) (Utilities|String|StringToName MapName) true "listen"))
    (:OnFailure
      (Development|PrintString "Failed session creation" true true "(R=1.000000,G=0.000000,B=0.000000,A=1.000000)" 1e+01))))

(event EventOnSessionInviteAccepted
  (params (LocalPlayerNum :type Integer) (PersonInvited :type BP%20Unique%20Net%20Id%20Structure) (SessionToJoin :type Blueprint%20Session%20Result%20Structure%20%28by%20ref%29))
  ;[0 0 0] INVITE
  (|JoinSession (Game|GetPlayerController 0) SessionToJoin))

(event EventOnSessionInviteReceived
  (params (LocalPlayerNum :type Integer) (PersonInviting :type BP%20Unique%20Net%20Id%20Structure) (AppId :type String) (SessionToJoin :type Blueprint%20Session%20Result%20Structure%20%28by%20ref%29))
  ;[0 0 0] INVITE
)

(event EventSavePlayerInfo
  (params (PlayerInfo :type S%20Player%20Info%20Structure))
  (Variables|Default|SetPlayerSteamInfo PlayerInfo))