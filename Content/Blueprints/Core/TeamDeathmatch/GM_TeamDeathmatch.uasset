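; Game mode for round-based Team Deathmatch that manages teams, spawning, round timing and match end.
; It tracks joined controllers, spawns red or blue characters at random team spawn points, and records teams in GameState and PlayerState.
; After a countdown, a looping timer runs the round clock; expiry freezes players, checks the winner, then returns to menu.
; An eliminated team concedes the round, leading to respawns until a two-point lead or round limit ends the match.
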(event Custom|Countdown
  ;[0 0 0] Countdown timer
  (if (not (Variables|Default|GetIsGameStarted?))
    (for _array_element (Variables|Default|GetPlayers)
      (Default|ShowCountdown _array_element))
    (Variables|Default|SetIsGameStarted? true)
    (Utilities|FlowControl|Delay 1e+01)
    (CallFunction|Unfreeze)))

(event Custom|Unfreeze
  ;[0 0 0] Freeze game
  (for _array_element (Variables|Default|GetPlayers)
    (Default|Unfreeze _array_element))
  (Variables|/Game/Blueprints/Core/TeamDeathmatch/GS_TeamDeathmatch.GS_TeamDeathmatch_C|SetCurrentTime (Variables|Default|GetGS_TeamDeathmatch) (Variables|Default|GetRoundTime))
  (bind _returnvalue (Utilities|Time|SetTimerbyEvent (delegate Custom|Count) 1.0 true))
  (CallFunction|ShowGameTimer))

(event Custom|ResultGame
  ;[0 0 0] End game - back to menu
  (CallFunction|BacktoMainMenu))

(event Custom|Respawn
  ;[0 0 0] Respawn players
  (for _array_element (Variables|Default|GetPlayers)
    (Default|RespawnPlayer _array_element)))

(event Custom|Count
  ;[0 0 0] Freeze game
  (bind _result (Math|Integer|DecrementInt (Variables|/Game/Blueprints/Core/TeamDeathmatch/GS_TeamDeathmatch.GS_TeamDeathmatch_C|GetCurrentTime (Variables|Default|GetGS_TeamDeathmatch)))
    (:%20%20
      (if (== _result 0)
        (Utilities|Time|PauseTimerbyHandle (stale Custom|Unfreeze _returnvalue))
        (CallFunction|Freeze)
        (CallFunction|CheckRoundWinner)
        (Utilities|FlowControl|Delay 5.0)
        (CallFunction|BacktoMainMenu)))))

(event Custom|ShowGameTimer
  ;[0 0 0] Countdown timer
  (for _array_element (Variables|Default|GetPlayers)
    (Default|ShowinGameTimer _array_element)))

(event Custom|Freeze
  ;[0 0 0] Freeze game
  (for _array_element (Variables|Default|GetPlayers)
    (Default|Freeze _array_element)))

(event Custom|BackToMainMenu
  ;[0 0 0] End game - back to menu
  (for _array_element (Variables|Default|GetPlayers)
    (Default|BacktoMainMenu _array_element)))

(event Custom|SpawnTeamA
  (params (PlayerController :type Player%20Controller%20Object%20Reference))
  (bind _teamaspawnpoints (Variables|Default|GetTeamASpawnPoints))
  (bind _playerstate (Variables|/Script/Engine.Controller|GetPlayerState PlayerController))
  ;[0 0 0] Spawn Team A - Get Position for Spawn
  (Class|BPIPC|SpawnPlayer(Message) PlayerController "/Game/Blueprints/Player/CH_Player_Red.CH_Player_Red_C" (Transformation|GetActorTransform (Utilities|Array|Get(acopy) _teamaspawnpoints (Math|Random|RandomIntegerinRange 0 (- (Utilities|Array|Length _teamaspawnpoints) 1)))))
  (if (Variables|Default|GetIsFirstRound?)
    (bind _asgs_team_deathmatch (Utilities|Casting|CastToGS_TeamDeathmatch (Game|GetGameState)))
    (Variables|Default|SetGS_TeamDeathmatch _asgs_team_deathmatch)
    (Utilities|Array|Add (Variables|/Game/Blueprints/Core/TeamDeathmatch/GS_TeamDeathmatch.GS_TeamDeathmatch_C|GetTeamA (Variables|Default|GetGS_TeamDeathmatch)) (PlayerState|GetPlayerName _playerstate))
    (Math|Integer|IncrementInt (Variables|/Game/Blueprints/Core/TeamDeathmatch/GS_TeamDeathmatch.GS_TeamDeathmatch_C|GetTeamASize (Variables|Default|GetGS_TeamDeathmatch))
      (:%20%20
        _))
    (else
      (Variables|/Game/Blueprints/Core/TeamDeathmatch/GS_TeamDeathmatch.GS_TeamDeathmatch_C|SetTeamASize (Variables|Default|GetGS_TeamDeathmatch) (Utilities|Array|Length (Variables|/Game/Blueprints/Core/TeamDeathmatch/GS_TeamDeathmatch.GS_TeamDeathmatch_C|GetTeamA (Variables|Default|GetGS_TeamDeathmatch))))))
  (bind _asps_team_deathmatch (Utilities|Casting|CastToPS_TeamDeathmatch _playerstate))
  (Variables|/Game/Blueprints/Core/TeamDeathmatch/PS_TeamDeathmatch.PS_TeamDeathmatch_C|SetTeam _asps_team_deathmatch "A"))

(event Custom|SpawnTeamB
  (params (PlayerController :type Player%20Controller%20Object%20Reference))
  (bind _playerstate (Variables|/Script/Engine.Controller|GetPlayerState PlayerController))
  (bind _teambspawnpoints (Variables|Default|GetTeamBSpawnPoints))
  ;[0 0 0] Spawn Team B - Get Position for Spawn
  (Class|BPIPC|SpawnPlayer(Message) PlayerController "/Game/Blueprints/Player/CH_Player_Blue.CH_Player_Blue_C" (Transformation|GetActorTransform (Utilities|Array|Get(acopy) _teambspawnpoints (Math|Random|RandomIntegerinRange 0 (- (Utilities|Array|Length _teambspawnpoints) 1)))))
  (if (Variables|Default|GetIsFirstRound?)
    (bind _asgs_team_deathmatch (Utilities|Casting|CastToGS_TeamDeathmatch (Game|GetGameState)))
    (Variables|Default|SetGS_TeamDeathmatch _asgs_team_deathmatch)
    (Utilities|Array|Add (Variables|/Game/Blueprints/Core/TeamDeathmatch/GS_TeamDeathmatch.GS_TeamDeathmatch_C|GetTeamB (Variables|Default|GetGS_TeamDeathmatch)) (PlayerState|GetPlayerName _playerstate))
    (Math|Integer|IncrementInt (Variables|/Game/Blueprints/Core/TeamDeathmatch/GS_TeamDeathmatch.GS_TeamDeathmatch_C|GetTeamBSize (Variables|Default|GetGS_TeamDeathmatch))
      (:%20%20
        _))
    (else
      (Variables|/Game/Blueprints/Core/TeamDeathmatch/GS_TeamDeathmatch.GS_TeamDeathmatch_C|SetTeamBSize (Variables|Default|GetGS_TeamDeathmatch) (Utilities|Array|Length (Variables|/Game/Blueprints/Core/TeamDeathmatch/GS_TeamDeathmatch.GS_TeamDeathmatch_C|GetTeamB (Variables|Default|GetGS_TeamDeathmatch))))))
  (bind _asps_team_deathmatch (Utilities|Casting|CastToPS_TeamDeathmatch _playerstate))
  (Variables|/Game/Blueprints/Core/TeamDeathmatch/PS_TeamDeathmatch.PS_TeamDeathmatch_C|SetTeam _asps_team_deathmatch "B"))

(event Custom|CheckRoundWinner
  (bind _gs_teamdeathmatch (Variables|Default|GetGS_TeamDeathmatch))
  ;[0 0 0] Check winner team
  (if (== (Variables|/Game/Blueprints/Core/TeamDeathmatch/GS_TeamDeathmatch.GS_TeamDeathmatch_C|GetTeamASize _gs_teamdeathmatch) 0)
    (bind _result (Math|Integer|IncrementInt (Variables|/Game/Blueprints/Core/TeamDeathmatch/GS_TeamDeathmatch.GS_TeamDeathmatch_C|GetTeamBScores (Variables|Default|GetGS_TeamDeathmatch)))
      (:%20%20
        (if (> (- _result (Variables|/Game/Blueprints/Core/TeamDeathmatch/GS_TeamDeathmatch.GS_TeamDeathmatch_C|GetTeamAScores (Variables|Default|GetGS_TeamDeathmatch))) 1)
          (CallFunction|ResultGame)
          (else
            (for _array_element (Variables|Default|GetPlayers)
              (bind _asps_team_deathmatch (Utilities|Casting|CastToPS_TeamDeathmatch (Variables|/Script/Engine.Controller|GetPlayerState _array_element)))
              (if (Utilities|Enum|Equal(Enum) (Variables|/Game/Blueprints/Core/TeamDeathmatch/PS_TeamDeathmatch.PS_TeamDeathmatch_C|GetTeam _asps_team_deathmatch) "A")
                (Default|ShowWinnerWidget _array_element false)
                (else
                  (Default|ShowWinnerWidget _array_element true)))
              (Utilities|FlowControl|Delay 5.0)
              (CallFunction|CheckRound))))))
    (elif (== (Variables|/Game/Blueprints/Core/TeamDeathmatch/GS_TeamDeathmatch.GS_TeamDeathmatch_C|GetTeamBSize _gs_teamdeathmatch) 0)
      (bind _result_2 (Math|Integer|IncrementInt (Variables|/Game/Blueprints/Core/TeamDeathmatch/GS_TeamDeathmatch.GS_TeamDeathmatch_C|GetTeamAScores (Variables|Default|GetGS_TeamDeathmatch)))
        (:%20%20
          (if (> (- _result_2 (Variables|/Game/Blueprints/Core/TeamDeathmatch/GS_TeamDeathmatch.GS_TeamDeathmatch_C|GetTeamBScores (Variables|Default|GetGS_TeamDeathmatch))) 1)
            (CallFunction|ResultGame)
            (else
              (for _array_element_2 (Variables|Default|GetPlayers)
                (bind _asps_team_deathmatch_2 (Utilities|Casting|CastToPS_TeamDeathmatch (Variables|/Script/Engine.Controller|GetPlayerState _array_element_2)))
                (if (Utilities|Enum|Equal(Enum) (Variables|/Game/Blueprints/Core/TeamDeathmatch/PS_TeamDeathmatch.PS_TeamDeathmatch_C|GetTeam _asps_team_deathmatch_2) "B")
                  (Default|ShowWinnerWidget _array_element_2 false)
                  (else
                    (Default|ShowWinnerWidget _array_element_2 true)))
                (Utilities|FlowControl|Delay 5.0)
                (CallFunction|CheckRound)))))))))

(event Custom|CheckRound
  (bind _gs_teamdeathmatch (Variables|Default|GetGS_TeamDeathmatch))
  (bind _currentround (Variables|/Game/Blueprints/Core/TeamDeathmatch/GS_TeamDeathmatch.GS_TeamDeathmatch_C|GetCurrentRound _gs_teamdeathmatch))
  ;[0 0 0] Check round number
  (if (< _currentround 3)
    (Math|Integer|IncrementInt _currentround
      (:%20%20
        (Variables|/Game/Blueprints/Core/TeamDeathmatch/GS_TeamDeathmatch.GS_TeamDeathmatch_C|SetCurrentTime (Variables|Default|GetGS_TeamDeathmatch) (Variables|Default|GetRoundTime))
        (Variables|Default|SetIsFirstRound? false)
        (CallFunction|Respawn)))
    (else
      (CallFunction|ResultGame))))

(event EventBeginPlay
  ;[0 0 0] Begin play
  (Utilities|FlowControl|Sequence
    (:then_0
      (bind _outactors (Actor|GetAllActorsOfClass "/Game/Blueprints/Spawn_A.Spawn_A_C"))
      (Variables|Default|SetTeamASpawnPoints _outactors))
    (:then_1
      (bind _outactors_2 (Actor|GetAllActorsOfClass "/Game/Blueprints/Spawn_B.Spawn_B_C"))
      (Variables|Default|SetTeamBSpawnPoints _outactors_2))))

(event EventPostLogin
  (params (NewPlayer :type Player%20Controller%20Object%20Reference))
  ;[0 0 0] On Post Login
  (Class|BPIPC|ShowTeamSelection(Message) NewPlayer)
  (bind _aspc_team_deathmatch (Utilities|Casting|CastToPC_TeamDeathmatch NewPlayer))
  (Utilities|Array|Add (Variables|Default|GetPlayers) _aspc_team_deathmatch))

(fn ConstructionScript)