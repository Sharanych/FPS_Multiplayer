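; Player controller for Team Deathmatch that manages each player's UI, input modes and team spawning.
; It requests team spawns and respawns from GM_TeamDeathmatch, while SpawnPlayer creates the character and possesses it through a multicast event.
; Client events drive team selection and ammo display, alongside health, countdown, timer, held scoreboard and round result widgets.
; At match end it shows the game result, destroys the session and opens the main menu.
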(event Custom|ShowCountdown
  ;[0 0 0] Timers UI
  (Widget|SetVisibility (Variables|Default|GetHUD) "Hidden")
  (bind _returnvalue (UserInterface|CreateWidget "/Game/UI/W_Countdown.W_Countdown_C"))
  (UserInterface|Viewport|AddtoViewport _returnvalue 0)
  (Utilities|FlowControl|Delay 1e+01)
  (Widget|SetVisibility (Variables|Default|GetHUD) "Visible"))

(event Custom|Unfreeze
  ;[0 0 0] Freeze / Unfreeze
  (Input|SetInputModeGameOnly self))

(event Custom|CLIENT_SetMaxAmmoUI
  (params (MaxAmmo :type Integer))
  ;[0 0 0] Ammo UI
  (Default|SetMaxAmmo (Variables|Default|GetHUD) MaxAmmo))

(event Custom|StartRoundTimer
  ;[0 0 0] Start countdown timer
  (bind _asgm_team_deathmatch (Utilities|Casting|CastToGM_TeamDeathmatch (Game|GetGameMode)))
  (Default|Countdown _asgm_team_deathmatch))

(event Custom|CLIENT_UpdateAmmoUI
  (params (CurrentAmmo :type Integer))
  ;[0 0 0] Ammo UI
  (Default|UpdateAmmo (Variables|Default|GetHUD) CurrentAmmo))

(event Custom|RespawnPlayer
  (bind _self self)
  (bind _returnvalue (Pawn|GetControlledPawn _self))
  ;[0 0 0] Respawn
  (Utilities|IsValid _returnvalue
    (:Is%20Valid
      (Actor|DestroyActor _returnvalue))
    (:Is%20Not%20Valid
      _))
  (bind _asps_team_deathmatch (Utilities|Casting|CastToPS_TeamDeathmatch (Variables|GetPlayerState)))
  (if (Utilities|Enum|Equal(Enum) (Variables|/Game/Blueprints/Core/TeamDeathmatch/PS_TeamDeathmatch.PS_TeamDeathmatch_C|GetTeam _asps_team_deathmatch) "A")
    (CallFunction|RequestTeamASpawn)
    (else
      (CallFunction|RequestTeamBSpawn))))

(event Custom|MULTICAST_PossessPlayer
  (params (InPawn :type Pawn%20Object%20Reference))
  (bind _hud (Variables|Default|GetHUD))
  ;[0 0 0] Respawn
  (Pawn|Possess InPawn)
  (if (Pawn|IsLocalPlayerController self)
    (Utilities|IsValid _hud
      (:Is%20Valid
        (Default|ResetWidget _hud)
        (Widget|SetVisibility _hud "Visible")
        (CallFunction|Unfreeze self)))))

(event Custom|ShowInGameTimer
  ;[0 0 0] Timers UI
  (bind _returnvalue (UserInterface|CreateWidget "/Game/UI/W_InGameTimer.W_InGameTimer_C"))
  (UserInterface|Viewport|AddtoViewport _returnvalue 0))

(event Custom|Freeze
  ;[0 0 0] Freeze / Unfreeze
  (Input|SetInputModeUIOnly self 0 "DoNotLock"))

(event Custom|ShowWinnerWidget
  (params (IsWon? :type Boolean))
  ;[0 0 0] Round result UI
  (Widget|SetVisibility (Variables|Default|GetHUD) "Hidden")
  (bind _returnvalue (UserInterface|CreateWidget "/Game/UI/W_RoundResult.W_RoundResult_C" 0 IsWon?))
  (UserInterface|Viewport|AddtoViewport _returnvalue 0)
  (Utilities|FlowControl|Delay 5.0)
  (Widget|RemovefromParent _returnvalue)
  (Widget|SetVisibility (Variables|Default|GetHUD) "Visible"))

(event Custom|BackToMainMenu
  ;[0 0 0] Destroy session
  (Viewport|RemoveAllWidgets)
  (bind _returnvalue (UserInterface|CreateWidget "/Game/UI/W_GameResult.W_GameResult_C"))
  (UserInterface|Viewport|AddtoViewport _returnvalue 0)
  (Utilities|FlowControl|Delay 5.0)
  (|DestroySession self
    (:then
      (Game|OpenLevel(byName) "MenuMap"))))

(event Custom|RequestTeamASpawn
  ;[0 0 0] Teams Spawn
  (Default|SpawnTeamA (Variables|Default|GetGM_TeamDeathmatch) self))

(event Custom|RequestTeamBSpawn
  ;[0 0 0] Teams Spawn
  (Default|SpawnTeamB (Variables|Default|GetGM_TeamDeathmatch) self))

(event Custom|CLIENT_ShowTeamSelection
  ;[0 0 0] Team Selection UI
  (bind _returnvalue (UserInterface|CreateWidget "/Game/UI/W_TeamSelection.W_TeamSelection_C"))
  (bind _output_get (Variables|Default|SetTeamSelectionWidget _returnvalue))
  (UserInterface|Viewport|AddtoViewport _output_get 0)
  (Input|SetInputModeGameandUI self (Variables|Default|GetTeamSelectionWidget) "DoNotLock" true)
  (Variables|Default|SetbShowMouseCursor true))

(event Custom|CLIENT_RemoveTeamSelection
  ;[0 0 0] Team Selection UI
  (Widget|RemovefromParent (Variables|Default|GetTeamSelectionWidget))
  (Input|SetInputModeGameOnly self)
  (Variables|Default|SetbShowMouseCursor false))

(event EventTeamASpawn
  ;[0 0 0] Teams Spawn
  (CallFunction|RequestTeamASpawn))

(event EventTeamBSpawn
  ;[0 0 0] Teams Spawn
  (CallFunction|RequestTeamBSpawn))

(event EventBeginPlay
  ;[0 0 0] Begin play
  (bind _asgm_team_deathmatch (Utilities|Casting|CastToGM_TeamDeathmatch (Game|GetGameMode))
    (:then
      (Variables|Default|SetGM_TeamDeathmatch _asgm_team_deathmatch))
    (:CastFailed
      _))
  (if (Pawn|IsLocalPlayerController)
    (bind _returnvalue (UserInterface|CreateWidget "/Game/UI/W_HUD.W_HUD_C" self))
    (bind _output_get (Variables|Default|SetHUD _returnvalue))
    (UserInterface|Viewport|AddtoViewport _output_get 0)
    (Input|SetInputModeUIOnly self 0 "DoNotLock")))

(event EventShowTeamSelection
  ;[0 0 0] Team Selection UI
  (CallFunction|CLIENTShowTeamSelection))

(event EventSpawnPlayer
  (params (CharacterClass :type CH%20Player%20Class%20Reference) (Transform :type Transform))
  ;[0 0 0] Player Spawn
  (bind _returnvalue (Game|SpawnActorfromClass CharacterClass Transform "AdjustIfPossibleButAlwaysSpawn" 0 "" 0))
  (CallFunction|MULTICASTPossessPlayer _returnvalue)
  (if (Variables|/Game/Blueprints/Core/TeamDeathmatch/GM_TeamDeathmatch.GM_TeamDeathmatch_C|GetIsFirstRound? (Variables|Default|GetGM_TeamDeathmatch))
    (CallFunction|CLIENTRemoveTeamSelection)))

(event EventUpdateAmmoUI
  (params (Ammo :type Integer))
  ;[0 0 0] Ammo UI
  (CallFunction|CLIENTUpdateAmmoUI Ammo))

(event EventSetMaxAmmoUI
  (params (MaxAmmo :type Integer))
  ;[0 0 0] Ammo UI
  (CallFunction|CLIENTSetMaxAmmoUI MaxAmmo))

(event EventUpdateHealthUI
  (params (Health :type Float%20%28single-precision%29))
  ;[0 0 0] Health UI
  (Default|UpdateHealth (Variables|Default|GetHUD) Health))

(event Input|ActionEvents|InputActionShowTeamScoreboard
  (params (Key :type Key%20Structure :default "None"))
  ;[0 0 0] Team scoreboard
  (:Pressed
    (Utilities|IsValid (Variables|Default|GetTeamBoard)
      (:Is%20Not%20Valid
        (bind _returnvalue (UserInterface|CreateWidget "/Game/UI/W_TeamBoard.W_TeamBoard_C"))
        (bind _output_get (Variables|Default|SetTeamBoard _returnvalue))
        (UserInterface|Viewport|AddtoViewport _output_get 0))))
  (:Released
    (Utilities|IsValid (Variables|Default|GetTeamBoard)
      (:Is%20Valid
        (Widget|RemovefromParent (Variables|Default|GetTeamBoard))
        (Variables|Default|SetTeamBoard 0)))))

(fn ConstructionScript)

(fn GetHUDRef
  (return (Variables|Default|GetHUD)))