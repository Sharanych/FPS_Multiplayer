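; PC_Menu is the player controller for the multiplayer menu, showing the W_MP_Menu widget on BeginPlay with UI-only input.
; When the Steam subsystem is present, it reads the player's name and requests their medium Steam avatar.
; Whether the avatar request succeeds or fails, it fills the PlayerInfo struct and passes it to the Game Instance through SavePlayerInfoMessage.
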(event Custom|ShowMPMenu
  (bind _returnvalue (UserInterface|CreateWidget "/Game/UI/W_MP_Menu.W_MP_Menu_C"))
  (UserInterface|Viewport|AddtoViewport _returnvalue 0)
  (Input|SetInputModeUIOnly self _returnvalue "DoNotLock"))

(event EventBeginPlay
  (bind _playerinfo (Variables|Default|GetPlayerInfo))
  (CallFunction|ShowMPMenu)
  (if (Class|AdvancedSessionsLibrary|HasOnlineSubsystem "STEAM")
    (Variables|Default|SetPlayerName (Utilities|Text|ToText(String) (Class|AdvancedSessionsLibrary|GetPlayerName self)))
    (bind _returnvalue (Class|AdvancedSteamFriendsLibrary|GetSteamFriendAvatar (Class|AdvancedSessionsLibrary|GetUniqueNetID self) "SteamAvatar_Medium")
      (:OnSuccess
        _)
      (:OnFailure
        _))
    (Utilities|Struct|SetmembersinS_PlayerInfo _playerinfo (Variables|Default|GetPlayerName) _returnvalue)
    (Class|BPIGameInstanceMP|SavePlayerInfo(Message) (Game|GetGameInstance) _playerinfo)))

(fn ConstructionScript)