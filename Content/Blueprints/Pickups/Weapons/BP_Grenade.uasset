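; BP_Grenade is a grenade actor that explodes as soon as anything begins overlapping its Sphere component.
; On the authority only, the overlap applies radial damage around the grenade's location, triggers the explosion effects and destroys the actor.
; A multicast event spawns the explosion particle and plays the sound at that location, keeping damage server-side while replicating the cosmetics.
; The overlap has no actor filter or fuse delay.
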(event OnComponentBeginOverlap(Sphere)
  (params (OverlappedComponent :type Primitive%20Component%20Object%20Reference) (OtherActor :type Actor%20Object%20Reference) (OtherComp :type Primitive%20Component%20Object%20Reference) (OtherBodyIndex :type Integer) (bFromSweep :type Boolean) (SweepResult :type Hit%20Result%20Structure%20%28by%20ref%29))
  (Networking|SwitchHasAuthority
    (:Authority
      (Game|Damage|ApplyRadialDamage (Variables|Default|GetBaseDamage) (Transformation|GetActorLocation) 7e+02 "/Script/Engine.DamageType" 0 self 0 false "ECC_Visibility")
      (CallFunction|MULTICASTSpawnEffects "/Game/Environment/Weapons/MilitaryWeapSilver/FX/P_Grenade_Explosion_01.P_Grenade_Explosion_01" (Transformation|GetActorLocation) "/Game/Environment/Weapons/MilitaryWeapSilver/Sound/GrenadeLauncher/Cues/GrenadeLauncher_Explosion_Cue.GrenadeLauncher_Explosion_Cue")
      (Actor|DestroyActor))))

(event Custom|MULTICAST_SpawnEffects
  (params (EmitterTemplate :type Particle%20System%20Object%20Reference) (Location :type Vector) (Sound :type Sound%20Base%20Object%20Reference))
  (Effects|SpawnEmitteratLocation EmitterTemplate Location)
  (Audio|PlaySoundatLocation Sound Location "0, 0, 0" 1.0 1.0 0.0 0 0 0))

(fn ConstructionScript)