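; BP_Weapon_GrenedeLauncher is a grenade launcher weapon pickup Blueprint that handles server-side firing.
; On fire it decrements the clip ammo and, while the count is not negative, updates the owner's ammo UI and multicasts a muzzle flash effect attached to the skeletal mesh.
; The fire graph shown spawns no projectile, and the construction script only calls the parent's.
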(event EventSERVERFireWeapon
  (bind _result (Math|Integer|DecrementInt (Variables|Default|GetAmmoInClip))
    (:%20%20
      (if (>= _result 0)
        (Class|BPIMPCharacter|UpdateAmmoUI(Message) (Components|GetOwner) _result)
        (CallFunction|MULTICASTWeaponEffects (Variables|Default|GetShootParticle) (Variables|Default|GetSK_Mesh) "MuzzleFlash")))))

(fn ConstructionScript
  (|CallParentFunction))