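; Base weapon actor for hitscan firearms, with server-side firing, ammo tracking and semi or automatic fire.
; Start fire shoots once, then automatic weapons repeat on a looping timer derived from fire rate until stopped or empty.
; Each shot updates the owner's ammo UI and line traces from the supplied player camera, using physical surface type to apply point damage, multiplied for headshots.
; Multicast events play muzzle and impact particles and sounds.
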(event Custom|MULTICAST_WeaponEffects
  (params (EmitterTemplate :type Particle%20System%20Object%20Reference) (AttachToComponent :type Scene%20Component%20Object%20Reference) (AttachPointName :type Name))
  ;[0 0 0] Effects
  (Effects|SpawnEmitterAttached EmitterTemplate AttachToComponent AttachPointName)
  (Audio|PlaySoundatLocation (Variables|Default|GetShootSound) (Transformation|GetActorLocation) "0, 0, 0" 1.0 1.0 0.0 0 0 0))

(event Custom|MULTICAST_HitEffects
  (params (EmitterTemplate :type Particle%20System%20Object%20Reference) (Location :type Vector) (Sound :type Sound%20Base%20Object%20Reference))
  ;[0 0 0] Effects
  (Effects|SpawnEmitteratLocation EmitterTemplate Location)
  (Audio|PlaySoundatLocation Sound (Transformation|GetActorLocation) "0, 0, 0" 1.0 1.0 0.0 0 0 0))

(event EventSERVERFireWeapon
  (bind _camera (Variables|Default|GetCamera))
  ;[0 0 0] Fire
  (bind _result (Math|Integer|DecrementInt (Variables|Default|GetAmmoInClip))
    (:%20%20
      (if (>= _result 0)
        (Class|BPIMPCharacter|UpdateAmmoUI(Message) (Components|GetOwner) _result)
        (CallFunction|MULTICASTWeaponEffects (Variables|Default|GetShootParticle) (Variables|Default|GetSK_Mesh) "MuzzleFlash")
        (bind _output_get (Variables|Default|SetCameraLocation (Transformation|GetWorldLocation _camera)))
        (Variables|Default|SetCameraRotation (Transformation|GetWorldRotation _camera))
        (bind (_outhit _returnvalue) (Collision|LineTraceByChannel _output_get (+ _output_get (* (Math|Vector|GetForwardVector (Variables|Default|GetCameraRotation)) (Variables|Damage|GetShootDistance))) "TraceTypeQuery1" true (Utilities|Array|MakeArray (Components|GetOwner) self) "None"))
        (if _returnvalue
          (switch Utilities|FlowControl|Switch|SwitchonEPhysicalSurface (Variables|/Script/Engine.PhysicalMaterial|GetSurfaceType (.PhysMat (Collision|BreakHitResult _outhit)))
            (:SurfaceType1
              ;;[0 0 0] Headshot
              (Utilities|ApplyDamage (.HitActor (Collision|BreakHitResult _outhit)) _outhit (* (Variables|Damage|GetBaseDamage) 4.0)
                (:out
                  (CallFunction|MULTICASTHitEffects (Variables|Damage|GetHeadshotParticle) (.ImpactPoint (Collision|BreakHitResult _outhit)) (Variables|Damage|GetHeadshotSound)))))
            (:SurfaceType2
              ;;[0 0 0] Body shoot
              (Utilities|ApplyDamage (.HitActor (Collision|BreakHitResult _outhit)) _outhit (Variables|Damage|GetBaseDamage)
                (:out
                  (CallFunction|MULTICASTHitEffects (Variables|Damage|GetBodyHitParticle) (.ImpactPoint (Collision|BreakHitResult _outhit)) (Variables|Damage|GetBodyHitSound)))))))
        (else
          (CallFunction|SERVERStopFire))))))

(event EventGetPlayerInfo
  (params (PlayerCamera :type Camera%20Component%20Object%20Reference) (Owner :type Character%20Object%20Reference))
  ;[0 0 0] Begin play
  (Variables|Default|SetCamera PlayerCamera)
  (Actor|SetOwner Owner))

(event EventSERVERStartFire
  ;[0 0 0] Fire
  (if (> (Variables|Default|GetAmmoInClip) 0)
    (CallFunction|SERVERFireWeapon)
    (if (Variables|Default|GetIsAutomatic?)
      (bind _returnvalue (Utilities|Time|SetTimerbyEvent (delegate EventSERVERFireWeapon) (Variables|Default|GetTimeBetweenShots) true))
      (Variables|Default|SetFiringTimer _returnvalue))))

(event EventSERVERStopFire
  ;[0 0 0] Fire
  (Utilities|Time|ClearandInvalidateTimerbyHandle (Variables|Default|GetFiringTimer)))

(event EventBeginPlay
  ;[0 0 0] Begin play
  (|CallParentFunction)
  (Variables|Default|SetTimeBetweenShots (/ 6e+01 (Variables|Default|GetFireRate))))

(fn ConstructionScript
  (|CallParentFunction))

(fn GetAmmoInfo
  (return (Variables|Default|GetAmmoInClip) (Variables|Default|GetMaxAmmo)))