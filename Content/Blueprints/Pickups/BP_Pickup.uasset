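; BP_Pickup is a base pickup actor for weapons, exposing weapon type, blend space, ammo info, pickup state and a self reference through getters.
; Fire, start-fire and stop-fire events forward to server events left empty here, and ammo info returns zeros.
; Other events disable the sphere's collision, clear the pickup flag or destroy the actor.
; The sphere overlap handler is empty, with its player pickup-message logic left disconnected.
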(event OnComponentBeginOverlap(Sphere)
  (params (OverlappedComponent :type Primitive%20Component%20Object%20Reference) (OtherActor :type Actor%20Object%20Reference) (OtherComp :type Primitive%20Component%20Object%20Reference) (OtherBodyIndex :type Integer) (bFromSweep :type Boolean) (SweepResult :type Hit%20Result%20Structure%20%28by%20ref%29))
  ;[1 0 0] Not use
)

(event Custom|SERVER_RemovePickup
  ;[0 0 0] Remove pickup
  (Actor|DestroyActor))

(event Custom|SERVER_DisableCollision
  ;[0 0 0] Remove pickup
  (Collision|SetCollisionEnabled (Variables|Default|GetSphere) "NoCollision"))

(event Custom|SERVER_FireWeapon
  ;[0 0 0] OVERRIDEN EVENTS
)

(event Custom|SERVER_StartFire
  ;[0 0 0] OVERRIDEN EVENTS
)

(event Custom|SERVER_StopFire
  ;[0 0 0] OVERRIDEN EVENTS
)

(event EventFireWeapon
  ;[0 0 0] OVERRIDEN EVENTS
  (CallFunction|SERVERFireWeapon))

(event EventStartFire
  ;[0 0 0] OVERRIDEN EVENTS
  (CallFunction|SERVERStartFire))

(event EventStopFire
  ;[0 0 0] OVERRIDEN EVENTS
  (CallFunction|SERVERStopFire))

(event EventDisableCollision
  ;[0 0 0] Remove pickup
  (Collision|SetCollisionEnabled (Variables|Default|GetSphere) "NoCollision")
  (Variables|Default|SetCanBePickup? false))

(fn ConstructionScript)

(fn BlendSpaceIndex
  (return (Variables|Default|GetBlendspace)))

(fn GetAmmoInfo
  (return 0 0))

(fn GetPickupState
  (return (Variables|Default|GetCanBePickup?)))

(fn GetWeaponType
  (return (Variables|Default|GetWeaponType)))

(fn PickupRef
  (return self))